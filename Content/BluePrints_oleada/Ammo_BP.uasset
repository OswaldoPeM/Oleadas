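; Ammo pickup actor that refills the player's ammunition when the E key is pressed.
; A Box overlap enables input on the actor for the first player controller, and ending the overlap disables it, without checking which actor overlaps.
; Pressing E adds a random amount to the FPS_Character's Municion variable and destroys the pickup.
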(event `self.Box.OnComponentBeginOverlap`
  (params (OverlappedComponent :type "PrimitiveComponent Object Reference") (OtherActor :type "Actor Object Reference") (OtherComp :type "PrimitiveComponent Object Reference") (OtherBodyIndex :type Integer) (bFromSweep :type Boolean) (SweepResult :type "HitResult Structure (by ref)"))
  (`self.EnableInput` (`GameplayStatics.GetPlayerController` 0)))

(event `self.Box.OnComponentEndOverlap`
  (params (OverlappedComponent :type "PrimitiveComponent Object Reference") (OtherActor :type "Actor Object Reference") (OtherComp :type "PrimitiveComponent Object Reference") (OtherBodyIndex :type Integer))
  (`self.DisableInput` (`GameplayStatics.GetPlayerController` 0)))

(event `Key|E`
  (params (Key :type "Key Structure"))
  (:`Pressed`
    (bind _asfps_character (cast `/Game/FirstPersonBP/Blueprints/FPS_Character` (`GameplayStatics.GetPlayerPawn` 0)))
    (set `/Game/FirstPersonBP/Blueprints/FPS_Character.municion` (+ (`/Game/FirstPersonBP/Blueprints/FPS_Character.municion` _asfps_character) (`KismetMathLibrary.RandomIntegerInRange` 30 60)) _asfps_character)
    (`self.K2_DestroyActor`)))

(fn `UserConstructionScript`)