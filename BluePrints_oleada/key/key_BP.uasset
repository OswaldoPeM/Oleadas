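; A key pickup actor that the player collects by walking into its box trigger.
; Tick accumulates time and spins the worn key mesh continuously around its yaw axis.
; On overlap with FPS_Character, it increments that character's Key count, plays a bell sound at the key's location and destroys itself.
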(event `self.ReceiveTick`
  (params (DeltaSeconds :type "Float (single-precision)"))
  (bind _time (`self.time`))
  (set `self.time` (+ DeltaSeconds _time))
  (`SceneComponent.K2_SetRelativeRotation` (`self.Worn_Key`) (`KismetMathLibrary.MakeRotator` 0.0 0.0 (* 500 _time)) false false))

(event `self.Box.OnComponentBeginOverlap`
  (params (OverlappedComponent :type "PrimitiveComponent Object Reference") (OtherActor :type "Actor Object Reference") (OtherComp :type "PrimitiveComponent Object Reference") (OtherBodyIndex :type Integer) (bFromSweep :type Boolean) (SweepResult :type "HitResult Structure (by ref)"))
  (bind _asfps_character (cast `/Game/FirstPersonBP/Blueprints/FPS_Character` OtherActor))
  (set `/Game/FirstPersonBP/Blueprints/FPS_Character.key` (+ (`/Game/FirstPersonBP/Blueprints/FPS_Character.key` _asfps_character) 1) _asfps_character)
  (`GameplayStatics.SpawnSoundAtLocation` "/Game/BluePrints_oleada/key/Pinball_Bell01.Pinball_Bell01" (`SceneComponent.K2_GetComponentLocation` (`self.Worn_Key`)) (struct) 1.0 1.0 0.0 null null)
  (`self.K2_DestroyActor`))

(fn `UserConstructionScript`)